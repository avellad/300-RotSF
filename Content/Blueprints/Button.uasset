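; Interactable push-button actor that the player presses with the Interact input while standing inside its collision volume.
; Collision overlaps with PlayerCharacter enable and disable the actor's input for player 0.
; Interact fires the TheButtonWasPushed event dispatcher, which the button binds itself to on BeginPlay.
; The bound event plays a click sound and runs a timeline that slides MoveableButton along its relative X.
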(event OnComponentBeginOverlap(collision)
  (params (OverlappedComponent :type Primitive%20Component%20Object%20Reference) (OtherActor :type Actor%20Object%20Reference) (OtherComp :type Primitive%20Component%20Object%20Reference) (OtherBodyIndex :type Integer) (bFromSweep :type Boolean) (SweepResult :type Hit%20Result%20Structure%20%28by%20ref%29))
  (Utilities|Casting|CastToPlayerCharacter OtherActor)
  (Input|EnableInput (Game|GetPlayerController 0)))

(event OnComponentEndOverlap(collision)
  (params (OverlappedComponent :type Primitive%20Component%20Object%20Reference) (OtherActor :type Actor%20Object%20Reference) (OtherComp :type Primitive%20Component%20Object%20Reference) (OtherBodyIndex :type Integer))
  (Utilities|Casting|CastToPlayerCharacter OtherActor)
  (Input|DisableInput (Game|GetPlayerController 0)))

(event Custom|CustomEvent_0
  (Audio|PlaySoundatLocation "/Engine/VREditor/Sounds/UI/Click_on_Button_Cue.Click_on_Button_Cue" (Transformation|GetActorLocation) "0, 0, 0" 1.0 1.0 0.0 0 0 0)
  (bind _relative_x (Timeline|Button%20Animation PlayFromStart)
    (:Update
      (Transformation|SetRelativeLocation (Variables|Default|Getmoveable%20button) (Math|Vector|MakeVector _relative_x 0.0 0.0) false false))))

(event EventBeginPlay
  (EventDispatchers|BindEventtoTheButtonWasPushed!!! (delegate Custom|CustomEvent_0)))

(event Input|ActionEvents|InputActionInteract
  (params (Key :type Key%20Structure :default "None"))
  (:Pressed
    (Default|CallTheButtonWasPushed!!!)))

(fn ConstructionScript)